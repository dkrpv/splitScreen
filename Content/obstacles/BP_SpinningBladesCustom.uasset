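; Spinning blade obstacle that slides between two configurable points and sends the first-person player back to a respawn point on contact.
; The construction script feeds the two relative locations and a duration into InterpToMovement, while Tick pitches the shuriken at a random per-instance speed.
; Capsule overlap or shuriken hit plays a damage sound and teleports the player to the TempleGameMode checkpoint, or a hard-coded start if none is reached.
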(event `self.ReceiveBeginPlay`
  (set `self.RotationAmount` (`KismetMathLibrary.RandomFloatInRange` 1.0 2.0))
  (`GameplayStatics.PlaySoundAtLocation` "/Game/Sounds/spinningblades.spinningblades" (`self.K2_GetActorLocation`) (struct) 0.2 1.0 0.0 null null null null))

(event `self.ReceiveTick`
  (params (DeltaSeconds :type "Float (single-precision)"))
  (`SceneComponent.K2_AddLocalRotation` (`self.shuriken`) (`KismetMathLibrary.MakeRotator` 0.0 (`self.RotationAmount`)) false false))

(event `self.Capsule.OnComponentBeginOverlap`
  (params (OverlappedComponent :type "PrimitiveComponent Object Reference") (OtherActor :type "Actor Object Reference") (OtherComp :type "PrimitiveComponent Object Reference") (OtherBodyIndex :type Integer) (bFromSweep :type Boolean) (SweepResult :type "HitResult Structure (by ref)"))
  (if (== (`GameplayStatics.GetObjectClass` OtherActor) "/Game/FirstPerson/Blueprints/BP_FirstPersonCharacter.BP_FirstPersonCharacter_C")
    (`GameplayStatics.PlaySound2D` "/Game/Sounds/damage.damage" 1.0 1.0 0.0 null null)
    (bind _astemple_game_mode (cast `/Game/Blueprints/TempleGameMode` (`GameplayStatics.GetGameMode`)))
    (if (`/Game/Blueprints/TempleGameMode.FirstCheckPoint` _astemple_game_mode)
      (`self.K2_TeleportTo` :`self` OtherActor :`DestLocation` (`/Game/Blueprints/TempleGameMode.respawnLocation` _astemple_game_mode))
      (else
        (`self.K2_TeleportTo` :`self` OtherActor :`DestLocation` (810.0 410.0 92.0))))))

(event `self.shuriken.OnComponentHit`
  (params (HitComponent :type "PrimitiveComponent Object Reference") (OtherActor :type "Actor Object Reference") (OtherComp :type "PrimitiveComponent Object Reference") (NormalImpulse :type "Vector Structure") (Hit :type "HitResult Structure (by ref)"))
  (if (== (`GameplayStatics.GetObjectClass` OtherActor) "/Game/FirstPerson/Blueprints/BP_FirstPersonCharacter.BP_FirstPersonCharacter_C")
    (`GameplayStatics.PlaySound2D` "/Game/Sounds/damage.damage" 1.0 1.0 0.0 null null)
    (bind _astemple_game_mode (cast `/Game/Blueprints/TempleGameMode` (`GameplayStatics.GetGameMode`)))
    (if (`/Game/Blueprints/TempleGameMode.FirstCheckPoint` _astemple_game_mode)
      (`self.K2_TeleportTo` :`self` OtherActor :`DestLocation` (`/Game/Blueprints/TempleGameMode.respawnLocation` _astemple_game_mode))
      (else
        (`self.K2_TeleportTo` :`self` OtherActor :`DestLocation` (810.0 410.0 92.0))))))

(fn `DEATH(Deprecated)`
  (bind _astemple_game_mode (cast `/Game/Blueprints/TempleGameMode` (`GameplayStatics.GetGameMode`)))
  (if (`/Game/Blueprints/TempleGameMode.FirstCheckPoint` _astemple_game_mode)
    (bind _returnvalue (`GameplayStatics.GetActorOfClass` "/Game/FirstPerson/Blueprints/BP_FirstPersonCharacter.BP_FirstPersonCharacter_C"))
    (`self.K2_TeleportTo` :`self` _returnvalue :`DestLocation` (`/Game/Blueprints/TempleGameMode.respawnLocation` _astemple_game_mode))
    (else
      (`self.K2_TeleportTo` :`self` _returnvalue :`DestLocation` (810.0 410.0 92.0)))))

(fn `UserConstructionScript`
  (bind _interptomovement (`self.InterpToMovement`))
  (set `InterpToMovementComponent.ControlPoints` (`|MakeArray` (make `InterpControlPoint` (`self.Location1`)) (make `InterpControlPoint` (`self.Location2`))) _interptomovement)
  (set `InterpToMovementComponent.Duration` (`self.Speed(lower=faster)`) _interptomovement))