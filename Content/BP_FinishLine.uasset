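; BP_FinishLine is a finish line trigger that ends the game when its Box component is overlapped.
; BeginPlay hides the cursor and sets game-only input for player 0.
; Any overlap sets LostGame, disables player 0's movement, shows WB_EndScreen with cursor and UI-only input, and removes player 1 along with its pawn.
; The overlap has no check on which actor entered.
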(event `self.ReceiveBeginPlay`
  (bind _returnvalue (`GameplayStatics.GetPlayerController` 0))
  (set `PlayerController.bShowMouseCursor` false _returnvalue)
  (`WidgetBlueprintLibrary.SetInputMode_GameOnly` _returnvalue))

(event `self.Box.OnComponentBeginOverlap`
  (params (OverlappedComponent :type "PrimitiveComponent Object Reference") (OtherActor :type "Actor Object Reference") (OtherComp :type "PrimitiveComponent Object Reference") (OtherBodyIndex :type Integer) (bFromSweep :type Boolean) (SweepResult :type "HitResult Structure (by ref)"))
  (bind _returnvalue (`GameplayStatics.GetPlayerController` 0))
  (set `self.LostGame` true)
  (`CharacterMovementComponent.DisableMovement` (`Character.CharacterMovement` (`GameplayStatics.GetPlayerCharacter` 0)))
  (bind _returnvalue_2 (`|CreateWidget` "/Game/WB_EndScreen.WB_EndScreen_C"))
  (`UserWidget.AddToViewport` _returnvalue_2 0)
  (set `PlayerController.bShowMouseCursor` true _returnvalue)
  (`WidgetBlueprintLibrary.SetInputMode_UIOnlyEx` _returnvalue _returnvalue_2)
  (`GameplayStatics.RemovePlayer` (`GameplayStatics.GetPlayerController` 1) true))

(fn `UserConstructionScript`)